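; BP_Deactivate is an interactable maze actor that disables traps by type when the Interact event fires.
; Its TrapName selects stake, swing or poison traps, and every actor of that Blueprint class in the level is destroyed.
; The deactivator then destroys itself.
; The construction script applies the Material variable to the second material slot of its Object component.
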(event `/Game/Maze/BPI_State.Interact`
  (if (== (`self.TrapName`) "Stake")
    (bind _outactors (`GameplayStatics.GetAllActorsOfClass` "/Game/Maze/BP_Stakes.BP_Stakes_C"))
    (for _array_element _outactors
      (`self.K2_DestroyActor` _array_element))
    (`self.K2_DestroyActor`)
    (elif (== (`self.TrapName`) "Swing")
      (bind _outactors_2 (`GameplayStatics.GetAllActorsOfClass` "/Game/Maze/BP_Swing.BP_Swing_C"))
      (for _array_element_2 _outactors_2
        (`self.K2_DestroyActor` _array_element_2))
      (`self.K2_DestroyActor`)
      (elif (== (`self.TrapName`) "Poison")
        (bind _outactors_3 (`GameplayStatics.GetAllActorsOfClass` "/Game/Maze/BP_Poison.BP_Poison_C"))
        (for _array_element_3 _outactors_3
          (`self.K2_DestroyActor` _array_element_3))
        (`self.K2_DestroyActor`)))))

(fn `UserConstructionScript`
  (`PrimitiveComponent.SetMaterial` (`self.Object`) 1 (`self.Material`)))