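; Maze game mode that runs the round clock and fails the run when time runs out.
; On BeginPlay it adds the W_UI widget, resets gold and starts a looping one-second timer that increments Time and broadcasts TimeChanged.
; At the time limit it sets Failed and calls FailedClockStop, which pauses the clock and broadcasts LightChanged.
; A separate WonClockStop event only pauses the clock.
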(event `FailedClockStop`
  (`KismetSystemLibrary.K2_PauseTimerHandle` (stale `self.ReceiveBeginPlay` _returnvalue_2))
  (`self.LightChanged`))

(event `self.ReceiveBeginPlay`
  (bind _returnvalue (`|CreateWidget` "/Game/Maze/W_UI.W_UI_C"))
  (`UserWidget.AddToViewport` _returnvalue 0)
  (set `self.CurrentGold` 0)
  (bind _returnvalue_2 (`KismetSystemLibrary.K2_SetTimer` null "Clock" 1.0 true)))

(event `WonClockStop`
  (`KismetSystemLibrary.K2_PauseTimerHandle` (stale `self.ReceiveBeginPlay` _returnvalue_2)))

(event `Clock`
  (bind _result (`/Engine/EditorBlueprintResources/StandardMacros.IncrementInt` (`self.Time`))
    (:`  `
      (`self.TimeChanged` _result)
      (if (== (`self.Time`) 100)
        (set `self.Failed` true)
        (`KismetSystemLibrary.PrintString` "Time is up!")
        (`self.FailedClockStop`)))))

(fn `UserConstructionScript`)