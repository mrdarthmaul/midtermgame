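; BP_Cell is a modular maze cell actor that builds its own floor, walls, ceiling and light.
; The construction script sizes the floor from GridSize, then adds static mesh pieces for each enabled wall or ceiling flag, scaled through SizeToCubeScale at hardcoded offsets.
; A centered point light with configurable color is added when LightIntensity is above zero.
; BeginPlay only caches a reference to the GM_Maze game mode.
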(event `self.ReceiveBeginPlay`
  (bind _asgm_maze (cast `/Game/Maze/GM_Maze` (`GameplayStatics.GetGameMode`)))
  (set `self.As GM Maze` _asgm_maze))

(fn `UserConstructionScript`
  (locals (WallThickness :type "Float (double-precision)") (WallLength :type "Float (double-precision)"))
  (bind _walllength (`local.WallLength`))
  (bind _gridsize (`self.GridSize`))
  (bind _returnvalue (* (`local.WallLength`) 0.5))
  (set `local.WallThickness` (* _gridsize 0.1))
  (set `local.WallLength` _gridsize)
  (`SceneComponent.SetRelativeScale3D` (`self.Floor`) (`self.SizeToCubeScale` (`KismetMathLibrary.MakeVector` _walllength _walllength (`local.WallThickness`))))
  (`|ExecutionSequence`
    (:`then_0`
      (if (`self.LeftWall`)
        (`AddComponent|NODE_AddStaticMeshComponent-0` :`RelativeTransform` (`KismetMathLibrary.MakeTransform` (0.0 0.0 50.0) (struct) (`self.SizeToCubeScale` (`KismetMathLibrary.MakeVector` (`local.WallLength`) (`local.WallThickness`) (`self.WallHeight`)))))))
    (:`then_1`
      (if (`self.RightWall`)
        (`AddComponent|NODE_AddStaticMeshComponent-2` :`RelativeTransform` (`KismetMathLibrary.MakeTransform` (0.0 450.0 50.0) (struct) (`self.SizeToCubeScale` (`KismetMathLibrary.MakeVector` (`local.WallLength`) (`local.WallThickness`) (`self.WallHeight`)))))))
    (:`then_2`
      (if (`self.BottomWall`)
        (`AddComponent|NODE_AddStaticMeshComponent-3` :`RelativeTransform` (`KismetMathLibrary.MakeTransform` (50.0 0.0 50.0) (struct :`Yaw` 90.0) (`self.SizeToCubeScale` (`KismetMathLibrary.MakeVector` (`local.WallLength`) (`local.WallThickness`) (`self.WallHeight`)))))))
    (:`then_3`
      (if (`self.TopWall`)
        (`AddComponent|NODE_AddStaticMeshComponent-4` :`RelativeTransform` (`KismetMathLibrary.MakeTransform` (500.0 0.0 50.0) (struct :`Yaw` 90.0) (`self.SizeToCubeScale` (`KismetMathLibrary.MakeVector` (`local.WallLength`) (`local.WallThickness`) (`self.WallHeight`)))))))
    (:`then_4`
      (if (`self.Ceiling`)
        (`AddComponent|NODE_AddStaticMeshComponent-5` :`RelativeTransform` (`KismetMathLibrary.MakeTransform` (500.0 0.0 600.0) (struct :`Yaw` 90.0 :`Roll` 90.0) (`self.SizeToCubeScale` (`KismetMathLibrary.MakeVector` (`local.WallLength`) (`local.WallThickness`) (`self.WallHeight`)))))))
    (:`then_5`
      (if (> (`self.LightIntensity`) 0.0)
        (bind _returnvalue_2 (`AddComponent|NODE_AddPointLightComponent-1` :`RelativeTransform` (`KismetMathLibrary.MakeTransform` (`KismetMathLibrary.MakeVector` _returnvalue _returnvalue (* (`self.WallHeight`) 0.75)))))
        (bind _output_get (set `self.LightComp` _returnvalue_2))
        (`LightComponent.SetIntensity` _output_get (`self.LightIntensity`))
        (`LightComponent.SetLightColor` (`self.LightComp`) (`self.Light Color`) true)))))