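; BP_Door is a keyed maze door that slides from a start to an end position when the player has the matching key.
; On BeginPlay it caches the GM_Maze game mode, and Interact compares that mode's CurrentKey to the door's KeyNumber.
; A match plays the DoorMove timeline to lerp the Door's relative location, otherwise it prints a message.
; The construction script applies a configurable material to the Door.
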(event `self.ReceiveBeginPlay`
  (bind _asgm_maze (cast `/Game/Maze/GM_Maze` (`GameplayStatics.GetGameMode`)))
  (set `self.GameMode` _asgm_maze))

(event `/Game/Maze/BPI_State.Interact`
  (if (== (`/Game/Maze/GM_Maze.CurrentKey` (`self.GameMode`)) (`self.KeyNumber`))
    (bind (_direction _godown) (`Timeline|DoorMove`)
      (:`Update`
        (`SceneComponent.K2_SetRelativeLocation` (`self.Door`) (`KismetMathLibrary.VLerp` (`self.StartLocation`) (`self.EndLocation`) _godown) false false)))
    (else
      (`KismetSystemLibrary.PrintString` "You don't have the required key."))))

(fn `UserConstructionScript`
  (`PrimitiveComponent.SetMaterial` (`self.Door`) 0 (`self.Material`)))