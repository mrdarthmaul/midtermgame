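; BP_Trap is a maze trap actor that places itself at a random grid cell when play begins.
; It caches the GM_Maze game mode, then teleports to a random 500-unit step on a seven-by-seven grid offset from LocationX and LocationY, at fixed height.
; Overlapping an actor whose display name exactly matches "BP_Trap" re-rolls the position.
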(event `self.ReceiveBeginPlay`
  (bind _asgm_maze (cast `/Game/Maze/GM_Maze` (`GameplayStatics.GetGameMode`)))
  (set `self.As GM Maze` _asgm_maze)
  (`self.K2_SetActorLocation` (`KismetMathLibrary.MakeVector` (+ (`self.LocationX`) (* (`KismetMathLibrary.RandomIntegerInRange` 0 6) 500.0)) (+ (`self.LocationY`) (* (`KismetMathLibrary.RandomIntegerInRange` 0 6) 500.0)) 250.0) false true :!label _label))

(event `self.ReceiveActorBeginOverlap`
  (params (OtherActor :type "Actor Object Reference"))
  (if (`KismetStringLibrary.EqualEqual_StrStr` (`KismetSystemLibrary.GetDisplayName` OtherActor) "BP_Trap")
    (goto _label)))

(fn `UserConstructionScript`)