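; BP_Swing is a swinging trap for the maze that damages the player character on contact.
; Overlapping the Box trigger restarts the Rotate timeline from the start, which drives the pitch of the Trap component.
; Overlapping the Trap subtracts fixed damage from the Health held on the maze game mode and calls its HealthChanged notification.
; Both overlaps identify the character by comparing its display name to "BP_Char".
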(event `self.Box.OnComponentBeginOverlap`
  (params (OverlappedComponent :type "PrimitiveComponent Object Reference") (OtherActor :type "Actor Object Reference") (OtherComp :type "PrimitiveComponent Object Reference") (OtherBodyIndex :type Integer) (bFromSweep :type Boolean) (SweepResult :type "HitResult Structure (by ref)"))
  (if (== (`KismetSystemLibrary.GetDisplayName` OtherActor) "BP_Char")
    (bind (_direction _y) (`Timeline|Rotate` :!via `PlayFromStart`)
      (:`Update`
        (`SceneComponent.K2_SetRelativeRotation` (`self.Trap`) (`KismetMathLibrary.MakeRotator` 0.0 _y) false false)))))

(event `self.Trap.OnComponentBeginOverlap`
  (params (OverlappedComponent :type "PrimitiveComponent Object Reference") (OtherActor :type "Actor Object Reference") (OtherComp :type "PrimitiveComponent Object Reference") (OtherBodyIndex :type Integer) (bFromSweep :type Boolean) (SweepResult :type "HitResult Structure (by ref)"))
  (bind _as_gm_maze (`self.As GM Maze`))
  (if (== (`KismetSystemLibrary.GetDisplayName` OtherActor) "BP_Char")
    (bind _output_get (set `/Game/Maze/GM_Maze.Health` (- (`/Game/Maze/GM_Maze.Health` _as_gm_maze) 3.0) _as_gm_maze))
    (`/Game/Maze/GM_Maze.HealthChanged` _as_gm_maze _output_get)))

(fn `UserConstructionScript`
  (`parent.UserConstructionScript`))